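; BP_LaserRaycast is a laser actor apparently meant to damage the first-person player.
; Every Tick it line traces on the Visibility channel between its StartPoint and EndPoint components, with debug drawing.
; The damage chain, which casts the hit actor to FirstPersonCharacter, lowers its Vida and prints it, is disconnected from execution, so the trace currently has no gameplay effect.
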(event `self.ReceiveTick`
  (params (DeltaSeconds :type "Float (single-precision)"))
  (bind _outhit (`KismetSystemLibrary.LineTraceSingle` :`Start` (`SceneComponent.K2_GetComponentLocation` (`self.StartPoint `)) :`End` (`SceneComponent.K2_GetComponentLocation` (`self.EndPoint`)) :`TraceChannel` "TraceTypeQuery1" :`DrawDebugType` "ForDuration")))

(fn `UserConstructionScript`)